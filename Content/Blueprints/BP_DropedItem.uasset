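; BP_DropedItem is a world pickup that puts an item in the player's hand when interacted with.
; It applies its Mesh variable to the static mesh on BeginPlay, and Interact calls Pickup.
; Pickup spawns an actor of class Type, stores it as BP_MyCharacter's CurrentItem, snaps it to PistolSocket on the first-person mesh, then destroys the pickup.
; Any previous CurrentItem is overwritten without cleanup here.
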(event `self.ReceiveBeginPlay`
  (`StaticMeshComponent.SetStaticMesh` (`self.StaticMesh`) (`self.Mesh`)))

(event `/Game/Blueprints/Interfaces/Interactable.Interact`
  (`/Game/Blueprints/Interfaces/Pickable.Pickup`))

(event `/Game/Blueprints/Interfaces/Pickable.Pickup`
  (bind _returnvalue (`GameplayStatics.GetPlayerPawn` 0))
  (bind _asbp_my_character (cast `/Game/Blueprints/BP_MyCharacter` _returnvalue))
  (bind _returnvalue_2 (`|SpawnActorFromClass` (`self.Type`) (`self.GetTransform` _returnvalue) "Undefined" "MultiplyWithRoot" null null))
  (bind _output_get (set `/Game/Blueprints/BP_MyCharacter.CurrentItem` _returnvalue_2 _asbp_my_character))
  (`self.K2_AttachToComponent` _output_get (`/Game/Blueprints/BP_MyCharacter.FirstPersonMesh` _asbp_my_character) "PistolSocket" "SnapToTarget" "SnapToTarget" "SnapToTarget" true)
  (`self.K2_DestroyActor`))

(fn `UserConstructionScript`)