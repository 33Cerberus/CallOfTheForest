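; Zombie enemy that patrols random navigable points until pawn sensing spots a pawn, then chases and attacks the player.
; AI MoveTo drives both movement loops, with chasing targeting player controller 0 and leading into an attack montage.
; A montage notify triggers a sphere overlap that damages nearby pawns.
; Damage plays a hit reaction and resumes the chase, while death stops movement, disables capsule collision and destroys the actor after a delay.
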(event `self.PawnSensing.OnSeePawn`
  (params (Pawn :type "Pawn Object Reference"))
  ;[0 1 0.9929] Setting Speed
  (set `self.SeePlayer` true)
  (`self.RunToPlayer`))

(event `self.ReceiveBeginPlay`
  ;[0.5945 1 0] BeginPlay
  (`self.Patrol`))

(event `Patrol`
  (if (not (`self.SeePlayer`))
    (bind _randomlocation (`NavigationSystemV1.K2_GetRandomLocationInNavigableRadius` (`self.K2_GetActorLocation`) 1000.0 null null))
    (`|AIMoveTo` self _randomlocation null 40.0
      (:`OnSuccess`
        (`self.Patrol`))
      (:`OnFail`
        (`self.Patrol`)))))

(event `RunToPlayer`
  ;[0.0138 0.151 0] Run To Player
  (if (not (`self.IsDeath`))
    (`|AIMoveTo` self (0.0 0.0 0.0) (`GameplayStatics.GetPlayerController` 0) 40.0
      (:`OnSuccess`
        (`self.AttackPlayer`))
      (:`OnFail`
        (`self.RunToPlayer`)))))

(event `AttackPlayer`
  ;[0.1714 0 1] Attack Player
  (`|PlayMontage` (`self.Mesh`) "/Game/Zombie/Animations/Montages/ZombieAttack_Montage.ZombieAttack_Montage"
    (:`OnCompleted`
      (`self.RunToPlayer`))
    (:`OnNotifyBegin`
      (`self.AttackPlayerLogic`))))

(event `self.ReceiveAnyDamage`
  (params (Damage :type "Float (single-precision)") (DamageType :type "DamageType Object Reference") (InstigatedBy :type "Controller Object Reference") (DamageCauser :type "Actor Object Reference"))
  ;[1 0.01055 0] Take Damage
  (if (not (`self.IsDeath`))
    (bind (_isdead _health) (`self.TakeDamage` Damage))
    (if _isdead
      (`self.Death`)
      (else
        (set `self.Health` _health)
        (`|PlayMontage` (`self.Mesh`) "/Game/Zombie/Animations/Montages/ZombieHitMontage.ZombieHitMontage"
          (:`then`
            (`self.RunToPlayer`)))))))

(event `Death`
  ;[0 0 0] Death
  (`self.Stop Movement`)
  (`|PlayMontage` (`self.Mesh`) "/Game/Zombie/Animations/Montages/ZombieDying_Montage.ZombieDying_Montage"
    (:`then`
      (`self.Disable`)
      (`KismetSystemLibrary.Delay` 10.0)
      (`self.K2_DestroyActor`))))

(fn `AttackPlayerLogic`
  ;[0 0.0615 1] AttackPlayerLogic
  (`GameplayStatics.PlaySoundAtLocation` "/Game/Sounds/AttackCue.AttackCue" (`self.K2_GetActorLocation`) (struct) 0.3 1.0 0.0 "/Game/MilitaryWeapSilver/Sound/Attenuation/WeaponShot_att.WeaponShot_att" null null null)
  (bind (_outactors _returnvalue) (`KismetSystemLibrary.SphereOverlapActors` (`SceneComponent.K2_GetComponentLocation` (`self.CapsuleComponent`)) 60.0 (`|MakeArray` "ObjectTypeQuery3" :!type "EObjectTypeQuery Enum") null (`|MakeArray` self :!type "Actor Object Reference")))
  (if _returnvalue
    (for _array_element _outactors
      (`GameplayStatics.ApplyDamage` _array_element 20.0 (`self.GetController`) self "/Script/Engine.DamageType"))))

(fn `Disable`
  ;[0 0 0] Disable
  (`PrimitiveComponent.SetCollisionEnabled` (`self.CapsuleComponent`) "NoCollision"))

(fn `Stop Movement`
  ;[0.08173 0 1] Stop Movement
  (set `self.IsDeath` true)
  (`NavMovementComponent.StopActiveMovement` (`self.CharacterMovement`)))

(fn `TakeDamage`
  (params (Damage :type "Float (double-precision)"))
  (returns (IsDead :type Boolean) (Health :type "Float (double-precision)"))
  (bind _returnvalue (- (`self.Health`) Damage))
  ;[1 0.008376 0] TakeDamage
  (return (<= _returnvalue 0.0) _returnvalue))

(fn `UserConstructionScript`)